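; BP_TextureSampler is a utility Blueprint that renders a source material into a render target, in an audio-reactive FX folder.
; DrawToRenderTarget checks that the render target and material are valid, clears the target to a set color, then draws the material into it, printing a message if either input is missing.
; An optional DrawOnTick flag makes Tick repeat the draw every frame.
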(event EventBeginPlay)

(event Collision|EventActorBeginOverlap
  (params (OtherActor :type Actor%20Object%20Reference)))

(event EventTick
  (params (DeltaSeconds :type Float%20%28single-precision%29))
  (if (Variables|Default|GetDrawOnTick)
    (CallFunction|DrawtoRenderTarget)))

(fn ConstructionScript)

(fn DrawtoRenderTarget
  (bind _sourcematerial (Variables|Default|GetSourceMaterial))
  (bind _rendertarget (Variables|Default|GetRenderTarget))
  (Utilities|IsValid _rendertarget
    (:Is%20Valid
      (Utilities|IsValid _sourcematerial
        (:Is%20Valid
          (Rendering|ClearRenderTarget2D _rendertarget (Variables|Default|GetClearColor))
          (Rendering|DrawMaterialtoRenderTarget _rendertarget _sourcematerial))
        (:Is%20Not%20Valid
          (Development|PrintString "Can not draw. Source material invalid"))))
    (:Is%20Not%20Valid
      (Development|PrintString "Can not draw. Render target invalid"))))